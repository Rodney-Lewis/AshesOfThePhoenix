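; A one-meter cube destructible that loses hit points when damaged and is removed from the world when they run out.
; A Destructible component hit from a FlyingPawn applies point damage to the hit result's actor, with the pawn as damage causer.
; AnyDamage subtracts truncated damage from ObjectHitPoints, prints the remainder and destroys the actor at zero or below.
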(event OnComponentHit(Destructible)
  (params (HitComponent :type Primitive%20Component%20Object%20Reference) (OtherActor :type Actor%20Object%20Reference) (OtherComp :type Primitive%20Component%20Object%20Reference) (NormalImpulse :type Vector :default "0, 0, 0") (Hit :type Hit%20Result%20Structure%20%28by%20ref%29))
  (bind (_bblockinghit _binitialoverlap _time _location _impactpoint _normal _impactnormal _physmat _hitactor) (Collision|BreakHitResult Hit))
  ;[1 1 1] Comment
  (bind _asflying_pawn (Utilities|Casting|CastToFlyingPawn OtherActor))
  (Game|Damage|ApplyPointDamage _hitactor (stale Game|Damage|EventAnyDamage Damage) _impactpoint Hit 0 _asflying_pawn "/Script/Engine.DamageType"))

(event Game|Damage|EventAnyDamage
  (params (Damage :type Float%20%28single-precision%29) (DamageType :type Damage%20Type%20Object%20Reference) (InstigatedBy :type Controller%20Object%20Reference) (DamageCauser :type Actor%20Object%20Reference))
  ;[1 1 1] Comment
  (bind _output_get (Variables|Default|SetObjectHitPoints (- (Variables|Default|GetObjectHitPoints) (Math|Float|Truncate Damage))))
  (Development|PrintString (Utilities|String|ToString(Integer) _output_get))
  (if (<= _output_get 0)
    (Actor|DestroyActor)))

(fn ConstructionScript)