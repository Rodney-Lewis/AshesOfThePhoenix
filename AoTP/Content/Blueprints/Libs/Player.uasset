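; Blueprint function library of player health helpers for the FlyingPawn: taking damage, checking death and regenerating health.
; Each function casts player pawn 0 to FlyingPawn and delegates the calculation to that pawn's Health member, passing in the pawn's own health values.
; Damage and regen write the result back to CurrentHealth, while IsDead returns the check's result.
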(fn TakeDamage
  (params (Damage :type Float%20%28single-precision%29))
  (bind _asflying_pawn (Utilities|Casting|CastToFlyingPawn (Game|Player|GetPlayerPawn 0)))
  (bind _newhealth (Default|TakeDamage (Variables|/Game/Blueprints/FlyingPawn.FlyingPawn_C|GetHealth _asflying_pawn) (Variables|/Game/Blueprints/FlyingPawn.FlyingPawn_C|GetCurrentHealth _asflying_pawn) Damage))
  (Variables|/Game/Blueprints/FlyingPawn.FlyingPawn_C|SetCurrentHealth _asflying_pawn _newhealth))

(fn IsDead
  (bind _asflying_pawn (Utilities|Casting|CastToFlyingPawn (Game|Player|GetPlayerPawn 0)))
  (bind _dead (Default|IsDead (Variables|/Game/Blueprints/FlyingPawn.FlyingPawn_C|GetHealth _asflying_pawn) (Variables|/Game/Blueprints/FlyingPawn.FlyingPawn_C|GetCurrentHealth _asflying_pawn)))
  (return _dead))

(fn RegenHealth
  (bind _asflying_pawn (Utilities|Casting|CastToFlyingPawn (Game|Player|GetPlayerPawn 0)))
  (bind _newhealth (Default|RegenHealth (Variables|/Game/Blueprints/FlyingPawn.FlyingPawn_C|GetHealth _asflying_pawn) (Variables|/Game/Blueprints/FlyingPawn.FlyingPawn_C|GetCurrentHealth _asflying_pawn) (Variables|/Game/Blueprints/FlyingPawn.FlyingPawn_C|GetMaximumHealth _asflying_pawn) (Variables|/Game/Blueprints/FlyingPawn.FlyingPawn_C|GetRegenRate _asflying_pawn)))
  (Variables|/Game/Blueprints/FlyingPawn.FlyingPawn_C|SetCurrentHealth _asflying_pawn _newhealth))