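; FlightHUD is a HUD Blueprint that draws a first-person crosshair texture at the middle of the screen.
; The DrawHUD event derives the position from half the screen size with a small fixed pixel offset.
; Tick casts the player pawn to FlyingPawn and reads its rotator, but nothing uses the result.
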(event EventDrawHUD
  (params (SizeX :type Integer) (SizeY :type Integer))
  ;[1 1 1] Crosshairs
  (Canvas|DrawTexture "/Game/Textures/FirstPersonCrosshair.FirstPersonCrosshair" (- (Math|Conversions|ToFloat(Integer) (/ SizeX 2)) 8.0) (- (Math|Conversions|ToFloat(Integer) (/ SizeY 2)) 8.0) 18.0 18.0 0.0 0.0 1.0 1.0 (Utilities|Struct|MakeLinearColor 1.0 1.0 1.0 1.0) "BLEND_Translucent" 1.0 true))

(event EventTick
  (params (DeltaSeconds :type Float%20%28single-precision%29))
  ;[1 1 1] Crosshairs
  (bind _asflying_pawn (Utilities|Casting|CastToFlyingPawn (Game|Player|GetPlayerPawn 0)))
  (bind _flightrotator (Default|GetRotator _asflying_pawn)))

(fn ConstructionScript)