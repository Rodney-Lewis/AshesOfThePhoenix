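; Health actor component that provides helper functions for damage, death checks and regeneration.
; It stores no result itself: each function takes health values as inputs and returns the result to the caller.
; Regeneration scales by world delta seconds and does not clamp, so it can slightly overshoot the maximum.
; The event graph is empty, so nothing runs on BeginPlay or Tick.
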(event EventBeginPlay)

(event EventTick
  (params (DeltaSeconds :type Float%20%28single-precision%29)))

(fn TakeDamage
  (params (CurrentHealth :type Float%20%28single-precision%29) (Damage :type Float%20%28single-precision%29))
  (return (- CurrentHealth Damage)))

(fn IsDead
  (params (Health :type Float%20%28single-precision%29))
  (return (<= Health 0.0)))

(fn RegenHealth
  (params (CurrentHealth :type Float%20%28single-precision%29) (MaximumHealth :type Float%20%28single-precision%29) (RegenFactor :type Float%20%28single-precision%29))
  (if (<= CurrentHealth MaximumHealth)
    (return (+ CurrentHealth (* RegenFactor (Utilities|Time|GetWorldDeltaSeconds))))
    (else
      (return CurrentHealth))))