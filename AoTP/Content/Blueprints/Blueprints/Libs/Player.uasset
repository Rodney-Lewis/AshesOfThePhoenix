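; Player function library that applies damage, checks death and regenerates health for the pawn of player index 0.
; Each function fetches and casts that pawn, then passes its health values to the matching Health function.
; TakeDamage and RegenHealth write the result back to CurrentHealth, while IsDead returns it.
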(fn TakeDamage
  (params (Damage :type Float%20%28single-precision%29))
  (Utilities|Casting|CastTo (Game|Player|GetPlayerPawn 0))
  (bind _newhealth (Default|TakeDamage (Variables|Default|GetHealth) (Variables|Default|GetCurrentHealth) Damage))
  (Variables|Default|SetCurrentHealth _newhealth))

(fn IsDead
  (Utilities|Casting|CastTo (Game|Player|GetPlayerPawn 0))
  (bind _dead (Default|IsDead (Variables|Default|GetHealth) (Variables|Default|GetCurrentHealth)))
  (return _dead))

(fn RegenHealth
  (Utilities|Casting|CastTo (Game|Player|GetPlayerPawn 0))
  (bind _newhealth (Default|RegenHealth (Variables|Default|GetHealth) (Variables|Default|GetCurrentHealth) (Variables|Default|GetMaximumHealth) (Variables|Default|GetRegenRate)))
  (Variables|Default|SetCurrentHealth 0 _newhealth))