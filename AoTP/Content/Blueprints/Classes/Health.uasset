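; Health Blueprint that provides three helper functions for damage, regeneration and death checks.
; Each works only on values passed in, so the caller holds the health state.
; TakeDamage subtracts damage without clamping, and IsDead reports whether health is at or below zero.
; RegenHealth adds one hundredth of the regen rate per call while below maximum, so the last step can overshoot it.
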(fn TakeDamage
  (params (CurrentHealth :type Float%20%28single-precision%29) (Damage :type Float%20%28single-precision%29))
  (return (- CurrentHealth Damage)))

(fn RegenHealth
  (params (CurrentHealth :type Float%20%28single-precision%29) (MaximumHealth :type Float%20%28single-precision%29) (RegenHealthRate :type Float%20%28single-precision%29))
  (if (< CurrentHealth MaximumHealth)
    (return (+ CurrentHealth (* RegenHealthRate 0.01)))
    (else
      (return CurrentHealth))))

(fn IsDead
  (params (CurrentHealth :type Float%20%28single-precision%29))
  (return (<= CurrentHealth 0.0)))