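; Destructible prop actor that tracks health and shatters when that health runs out.
; AnyDamage updates CurrentHealth through TakeDamage, checks IsDead, and prints the remaining health as debug output while the actor survives.
; On death, a DoOnce hides the cube, disables cube and cylinder collision, assigns a destructible mesh and applies a small radius damage to fracture it.
; The actor destroys itself after a delay.
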(event Game|Damage|EventAnyDamage
  (params (Damage :type Float%20%28single-precision%29) (DamageType :type Damage%20Type%20Object%20Reference) (InstigatedBy :type Controller%20Object%20Reference) (DamageCauser :type Actor%20Object%20Reference))
  (bind _destructiblecomponent (Variables|Default|GetDestructibleComponent))
  (bind _cube (Variables|Default|GetCube))
  ;[1 1 1] Take damage
  (bind _newhealth (CallFunction|TakeDamage (Variables|Default|GetCurrentHealth) Damage))
  (bind _output_get (Variables|Default|SetCurrentHealth _newhealth))
  (bind _dead (CallFunction|IsDead _output_get))
  (if _dead
    (Utilities|FlowControl|DoOnce false
      (:Completed
        (Rendering|SetVisibility _cube false false)
        (Collision|SetCollisionEnabled (Variables|Default|GetCylinder) "NoCollision")
        (Collision|SetCollisionEnabled _cube "NoCollision")
        (Class|DestructibleComponent|SetDestructibleMesh (Variables|Default|GetDestructibleComponent) "/Game/Meshes/Destructible1M_Cube_DM.Destructible1M_Cube_DM")
        (Class|DestructibleComponent|ApplyRadiusDamage _destructiblecomponent 0.5 (Transformation|GetWorldLocation _destructiblecomponent) 0.5 0.5 false)
        (Utilities|FlowControl|Delay 3e+01)
        (Actor|DestroyActor)))
    (else
      (Development|PrintString (Utilities|String|ToString(Float) _output_get) true true "(R=0.000000,G=0.660000,B=1.000000,A=1.000000)" 5.0))))

(fn ConstructionScript)